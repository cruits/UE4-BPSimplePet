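; BP_Projectile is an explosive projectile actor that damages whatever it hits.
; On BeginPlay it sets the capsule's physics velocity along its forward vector at Speed, then destroys itself after a short delay.
; On Hit it spawns an explosion particle at the impact point, applies fixed damage credited to the instigator's controller, and destroys itself.
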(event EventBeginPlay
  (bind _capsule (Variables|Default|GetCapsule))
  ;[1 1 1] 发射物运动
  (Physics|SetPhysicsLinearVelocity _capsule (* (Math|Vector|GetForwardVector (Transformation|GetWorldRotation _capsule)) (Variables|Default|GetSpeed)) false "None")
  (Utilities|FlowControl|Delay 2.0)
  (Actor|DestroyActor))

(event Collision|EventHit
  (params (MyComp :type Primitive%20Component%20Object%20Reference) (Other :type Actor%20Object%20Reference) (OtherComp :type Primitive%20Component%20Object%20Reference) (bSelfMoved :type Boolean) (HitLocation :type Vector :default "0, 0, 0") (HitNormal :type Vector :default "0, 0, 0") (NormalImpulse :type Vector :default "0, 0, 0") (Hit :type Hit%20Result%20Structure%20%28by%20ref%29))
  ;[1 1 1] 碰撞设置
  (Effects|SpawnEmitteratLocation "/Game/StarterContent/Particles/P_Explosion.P_Explosion" HitLocation)
  (Game|Damage|ApplyDamage Other 1e+02 (Game|GetInstigatorController) self)
  (Actor|DestroyActor))

(fn ConstructionScript)