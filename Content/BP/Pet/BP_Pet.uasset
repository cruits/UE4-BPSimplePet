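; BP_Pet is a pet actor whose AI behavior tree is driven by its master and the master's enemy.
; On the server, BeginPlay waits briefly, then starts BPT_PetAI and writes Master to the Blackboard if valid.
; SetEmeny (server-only) and ClearEnemy set or clear the enemy key.
; Aim yaws the body and fully rotates the Sphere toward MasterEnemy, while ClientFire defers to the parent.
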(event Custom|SetEmeny
  (bind _masterenemy (Variables|Default|GetMasterEnemy))
  (bind _blackboard (Variables|Default|GetBlackboard))
  ;[1 1 1] 受到攻击，在黑板写入敌人
  (Networking|SwitchHasAuthority
    (:Authority
      (Utilities|IsValid _masterenemy
        (:Is%20Valid
          (Utilities|IsValid _blackboard
            (:Is%20Valid
              (AI|Components|Blackboard|SetValueasObject _blackboard (Utilities|Name|MakeLiteralName "Emeny") _masterenemy))))))))

(event Custom|Aim
  (bind _self self)
  (bind _masterenemy (Variables|Default|GetMasterEnemy))
  (bind _sphere (Variables|Default|GetSphere))
  (bind _returnvalue (Transformation|GetActorLocation _masterenemy))
  (bind _returnvalue_2 (Transformation|GetActorRotation _self))
  (bind (_roll _pitch) (Math|Rotator|BreakRotator _returnvalue_2))
  ;[1 1 1] 瞄准
  (Transformation|SetActorRotation _self (Math|Rotator|MakeRotator _roll _pitch (.Yaw (Math|Rotator|BreakRotator (Math|Rotator|FindLookatRotation (Transformation|GetActorLocation _self) _returnvalue)))))
  (Transformation|SetWorldRotation _sphere (Math|Rotator|FindLookatRotation (Transformation|GetWorldLocation _sphere) _returnvalue) false false))

(event Custom|ClearEnemy
  ;[1 1 1] 受到攻击，在黑板写入敌人
  (AI|Components|Blackboard|SetValueasObject (Variables|Default|GetBlackboard) (Utilities|Name|MakeLiteralName "Emeny") 0))

(event EventBeginPlay
  (bind _self self)
  (bind _master (Variables|Default|GetMaster))
  ;[1 1 1] 刚生成Pet
  (Networking|SwitchHasAuthority
    (:Authority
      (Utilities|FlowControl|Delay 1.0)
      (Utilities|IsValid _master
        (:Is%20Valid
          (AI|RunBehaviorTree (AI|GetAIController _self) "/Game/BP/Pet/BPT_PetAI.BPT_PetAI")
          (bind _output_get (Variables|Default|SetBlackboard (AI|GetBlackboard _self)))
          (AI|Components|Blackboard|SetValueasObject _output_get (Utilities|Name|MakeLiteralName "Master") _master))))))

(event EventClientFire
  ;[1 1 1] Fire
  (|CallParentFunction))

(fn ConstructionScript)